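; Projectile actor that launches along its forward vector with a trail particle effect and explodes on impact.
; On any hit it triggers the explosion, hides the mesh, stops the particles, disables collision and destroys itself after a short delay.
; Only hits on Player-tagged actors also play a ping sound, send PlayerHitMessage with a fixed value and zero the velocity.
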(event EventBeginPlay
  (bind _returnvalue (Transformation|GetActorForwardVector))
  (bind _returnvalue_2 (* _returnvalue 1e+03))
  (Variables|/Script/Engine.MovementComponent|SetVelocity (Variables|Default|GetProjectileMovement) (Math|Vector|MakeVector (.x _returnvalue_2) (.y _returnvalue_2) (.z _returnvalue_2)))
  (Components|Activation|Activate (Variables|Default|GetParticles) false))

(event Collision|EventHit
  (params (MyComp :type Primitive%20Component%20Object%20Reference) (Other :type Actor%20Object%20Reference) (OtherComp :type Primitive%20Component%20Object%20Reference) (bSelfMoved :type Boolean) (HitLocation :type Vector :default "0, 0, 0") (HitNormal :type Vector :default "0, 0, 0") (NormalImpulse :type Vector :default "0, 0, 0") (Hit :type Hit%20Result%20Structure%20%28by%20ref%29))
  (if (Actor|ActorHasTag Other "Player")
    (Components|Activation|Activate (Variables|Default|GetExplosion) false)
    (Audio|PlaySoundatLocation "/Engine/EngineSounds/1kSineTonePing.1kSineTonePing" (Transformation|GetActorLocation) "0, 0, 0" 1.0 1.0 0.0 0 0 0 0)
    (Class|IDamage|PlayerHit(Message) Other 5.0)
    (Variables|/Script/Engine.MovementComponent|SetVelocity (Variables|Default|GetProjectileMovement) "0, 0, 0")
    (Rendering|SetVisibility (Variables|Default|GetStaticMesh) false false)
    (Components|Activation|Deactivate (Variables|Default|GetParticles))
    (Collision|SetActorEnableCollision false)
    (Utilities|FlowControl|Delay 2.0)
    (Actor|DestroyActor)
    (else
      (Components|Activation|Activate (Variables|Default|GetExplosion) false)
      (Collision|SetActorEnableCollision false)
      (Rendering|SetVisibility (Variables|Default|GetStaticMesh) false false)
      (Components|Activation|Deactivate (Variables|Default|GetParticles))
      (Utilities|FlowControl|Delay 2.0)
      (Actor|DestroyActor))))

(fn ConstructionScript)