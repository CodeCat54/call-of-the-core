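; BP_EnemyShooter is an enemy actor that periodically fires a ring of projectiles around itself.
; BeginPlay starts a looping timer that calls Attack at a fixed interval.
; Attack divides a full circle by the Projectiles count and spawns a BP_Projectile at each yaw step, offset outward and facing away.
; The yaw steps are combined with the actor's rotation, so the pattern follows the enemy's orientation.
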(event EventBeginPlay
  (Utilities|Time|SetTimerbyFunctionName 0 "Attack" 2.0 true))

(fn ConstructionScript)

(fn Attack
  (for _index (range 0 (- (Variables|Default|GetProjectiles) 1))
    (Game|SpawnActorfromClass "/Game/Blueprints/BP_Projectile.BP_Projectile_C" (Math|Transform|MakeTransform (+ (Transformation|GetActorLocation) (* (Math|Vector|GetForwardVector (Math|Rotator|CombineRotators (Transformation|GetActorRotation) (Math|Rotator|MakeRotator 0.0 0.0 (* _index (/ 360 (Variables|Default|GetProjectiles)))))) 100)) (Math|Rotator|CombineRotators (Transformation|GetActorRotation) (Math|Rotator|MakeRotator 0.0 0.0 (* _index (/ 360 (Variables|Default|GetProjectiles))))) "1.000000,1.000000,1.000000") "Undefined" "MultiplyWithRoot" 0 0)))