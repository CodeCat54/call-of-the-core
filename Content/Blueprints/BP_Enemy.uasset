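; Enemy that loses health each time it is shot and destroys itself at zero.
; Pawn sensing alternates on each sighting between a follow state and another enum state.
; Following sphere-traces ahead for pawns, switching state on an interface match and otherwise using AIMoveTo toward the seen pawn.
; The interface check is an unfinished placeholder for attacking, and the trace draws debug shapes.
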(event OnSeePawn(PawnSensing)
  (params (Pawn :type Pawn%20Object%20Reference))
  (Utilities|FlowControl|FlipFlop
    (:A
      (Variables|Default|SetEnemyStateEnum "NewEnumerator3")
      (CallFunction|FollowPlayer))
    (:B
      (Variables|Default|SetEnemyStateEnum "NewEnumerator1"))))

(event Custom|FollowPlayer
  (bind _returnvalue (Transformation|GetActorLocation))
  (bind _outhits (Collision|MultiSphereTraceForObjects _returnvalue (+ _returnvalue (* (Transformation|GetActorForwardVector) 1e+02)) 0.0 (Utilities|Array|MakeArray "ObjectTypeQuery3") false 0 "ForDuration"))
  (bind _array_element (Utilities|Array|ForEachLoopwithBreak _outhits :!label _label)
    (:LoopBody
      (if (Utilities|DoesObjectImplementInterface (.hitactor _array_element) 0)
        (Variables|Default|SetEnemyStateEnum "NewEnumerator0")
        (goto _label Break)))
    (:Completed
      (if (Utilities|Enum|NotEqual(Enum) (Variables|Default|GetEnemyStateEnum) "NewEnumerator0")
        (AI|AIMoveTo self "0, 0, 0" (stale OnSeePawn(PawnSensing) Pawn) 7e+01 false)))))

(event EventShot
  ;[1 1 1] Lose health when shot
  (Variables|Default|SetHealth (- (Variables|Default|GetHealth) 1e+01))
  (if (<= (Variables|Default|GetHealth) 0.0)
    (Actor|DestroyActor)))

(fn ConstructionScript)