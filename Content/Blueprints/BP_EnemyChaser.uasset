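; BP_EnemyChaser is a melee enemy that plays a spawn effect and montage, loses health when shot, and destroys itself at zero.
; Its AI loop moves to the player, turns, plays an attack montage with a timed Niagara slash, and retries on failure, but no event triggers it.
; That loop sets the attack state that gates weapon-overlap damage to actors tagged Player.
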(event OnComponentBeginOverlap(Weapon)
  (params (OverlappedComponent :type Primitive%20Component%20Object%20Reference) (OtherActor :type Actor%20Object%20Reference) (OtherComp :type Primitive%20Component%20Object%20Reference) (OtherBodyIndex :type Integer) (bFromSweep :type Boolean) (SweepResult :type Hit%20Result%20Structure%20%28by%20ref%29))
  ;[1 1 1] If hits player and in attack state, deal damage
  (if (Actor|ActorHasTag OtherActor "Player")
    (if (Utilities|Enum|Equal(Enum) (Variables|Default|GetEnemyStateEnum) "NewEnumerator0")
      (Class|IDamage|PlayerHit(Message) OtherActor 1e+01))))

(event EventBeginPlay
  (bind _spawneffect (Variables|Default|GetSpawnEffect))
  (Components|Activation|Activate (Variables|Default|GetSpawnEffect) false)
  (bind _returnvalue (Animation|PlayAnimMontage "/Game/Models/Knight/Animations/Montage_Spawn.Montage_Spawn" 1.0 "None"))
  (Utilities|FlowControl|Delay _returnvalue)
  (Components|Activation|Deactivate _spawneffect)
  (Rendering|ToggleVisibility _spawneffect false))

(event EventEnemyShot
  ;[1 1 1] Lose health when shot
  (Variables|Default|SetHealth (- (Variables|Default|GetHealth) 1e+01))
  (if (<= (Variables|Default|GetHealth) 0.0)
    (Actor|DestroyActor)))

(fn ConstructionScript)