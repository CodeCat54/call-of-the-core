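; Ranged enemy Blueprint that arms itself with a rifle when play begins.
; EquipWeapon spawns a BP_Weapon_Rifle, attaches it to the mesh's right-hand rifle socket, sets the wielding flag and fires the OnWeaponEquipped dispatcher.
; The Attack event is an empty stub, and the construction script only calls its parent.
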(event EventBeginPlay
  (CallFunction|EquipWeapon))

(event EventAttack)

(event EventEquipWeapon
  (bind _returnvalue (Game|SpawnActorfromClass "/Game/Weapons/BP_Weapon_Rifle.BP_Weapon_Rifle_C" (Math|Transform|MakeTransform "0, 0, 0") "Undefined" "MultiplyWithRoot" 0 0))
  (bind _output_get (Variables|Default|SetWeaponActor _returnvalue))
  (Transformation|AttachComponentToComponent _output_get (Variables|Character|GetMesh) "Hand_R_Rifle_Socket" "KeepRelative" "KeepRelative" "KeepRelative" true)
  (Variables|Default|SetIsWieldingWeapon true)
  (Default|CallOnWeaponEquipped))

(fn ConstructionScript
  (|CallParentFunction))