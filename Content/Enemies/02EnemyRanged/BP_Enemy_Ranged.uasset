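; Ranged enemy Blueprint that fights with a gun, offering rifle, shotgun, sniper and rocket attacks.
; EquipWeapon plays a draw montage, then spawns the gun and attaches it to the hand socket on the montage notify.
; Each attack event passes montage, damage and projectile settings to the BPCAttacks component, with randomised projectile speed except for sniper.
; Overrides also set enemy type, walk speeds, ideal range and anim class.
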(event Custom|ShotgunAttack
  (params (AttackTarget :type Actor%20Object%20Reference))
  ;[1 1 1] Shotgun attack
  (Default|ShotgunAttack (Variables|Default|GetBPC_Attacks) (Utilities|Struct|MakeS_AttackInfo AttackTarget "/Game/Enemies/02EnemyRanged/Animations/AM_RRanged_Fire.AM_RRanged_Fire" (Utilities|Struct|MakeS_DamageInfo (Variables|RifleAttack|GetRifleAttackDamage) "NewEnumerator2" "NewEnumerator0" false false true)) (Utilities|Array|Get(acopy) (Variables|Default|GetProjectilesArray) 6) (Math|Random|RandomFloatinRange (Variables|RifleAttack|GetRifleAttackMinSpeed) (Variables|RifleAttack|GetRifleAttackMaxSpeed)) 0.0 false "/Game/Sounds/SFX/SFX_Shotgun.SFX_Shotgun" (Variables|Default|GetSpreadTotalShots)))

(event Custom|SniperAttack
  (params (AttackTarget :type Actor%20Object%20Reference))
  ;[1 1 1] Sniper attack
  (Default|BasicMageAttack (Variables|Default|GetBPC_Attacks) (Utilities|Struct|MakeS_AttackInfo AttackTarget "/Game/Enemies/02EnemyRanged/Animations/AM_RRanged_Fire.AM_RRanged_Fire" (Utilities|Struct|MakeS_DamageInfo (Variables|SniperAttack|GetSniperAttackDamage) "NewEnumerator2" "NewEnumerator0" false false true)) (Utilities|Array|Get(acopy) (Variables|Default|GetProjectilesArray) 1) (Variables|SniperAttack|GetSniperAttackSpeed) 0.0 false))

(event Custom|RocketAttack
  (params (AttackTarget :type Actor%20Object%20Reference))
  ;[1 1 1] Rocket attack
  (Default|RocketAttack (Variables|Default|GetBPC_Attacks) (Utilities|Struct|MakeS_AttackInfo AttackTarget "/Game/Enemies/02EnemyRanged/Animations/AM_RRanged_Fire.AM_RRanged_Fire" (Utilities|Struct|MakeS_DamageInfo (Variables|RifleAttack|GetRifleAttackDamage) "NewEnumerator2" "NewEnumerator0" false false true)) (Utilities|Array|Get(acopy) (Variables|Default|GetProjectilesArray) 3) (Math|Random|RandomFloatinRange (Variables|RifleAttack|GetRifleAttackMinSpeed) (Variables|RifleAttack|GetRifleAttackMaxSpeed)) 0.0 false 2e+02 (Utilities|Struct|MakeS_DamageInfo (Variables|Default|GetRocketDamage) "NewEnumerator2")))

(event Custom|RifleAttack
  (params (AttackTarget :type Actor%20Object%20Reference))
  ;[1 1 1] Rifle attack
  (Default|RangedBarrage (Variables|Default|GetBPC_Attacks) (Utilities|Struct|MakeS_AttackInfo AttackTarget "/Game/Enemies/02EnemyRanged/Animations/AM_RRanged_Fire.AM_RRanged_Fire" (Utilities|Struct|MakeS_DamageInfo (Variables|RifleAttack|GetRifleAttackDamage) "NewEnumerator2" "NewEnumerator0" false false true)) (Utilities|Array|Get(acopy) (Variables|Default|GetProjectilesArray) 4) (Math|Random|RandomFloatinRange (Variables|RifleAttack|GetRifleAttackMinSpeed) (Variables|RifleAttack|GetRifleAttackMaxSpeed)) 0.0 false 0 0.2 (Variables|RifleAttack|GetRifleAttackTotalShots)))

(event EventBeginPlay
  ;[1 1 1] Initialise
  (|CallParentFunction))

(event EventEquipWeapon
  ;[1 1 1] Equip weapon
  (bind _notifyname (Animation|Montage|PlayMontage (Variables|Character|GetMesh) "/Game/Enemies/02EnemyRanged/Animations/AM_RRanged_DrawWeapon.AM_RRanged_DrawWeapon" 1.25)
    (:OnCompleted
      (Default|CallOnWeaponEquipped :!label _label))
    (:OnInterrupted
      (goto _label))
    (:OnNotifyBegin
      (switch name _notifyname
        (:Draw
          (bind _returnvalue (Game|SpawnActorfromClass "/Game/Weapons/BP_Weapon_Gun.BP_Weapon_Gun_C" (Math|Transform|MakeTransform "0, 0, 0" "0, 0, 0" "1.000000,1.000000,1.000000") "Undefined" "MultiplyWithRoot" 0 0 0))
          (bind _output_get (Variables|Default|SetWeaponActor _returnvalue))
          (Transformation|AttachComponentToComponent _output_get (Variables|Character|GetMesh) "Hand_R_Rifle_Socket" "KeepRelative" "KeepRelative" "KeepRelative" true)
          (Variables|Default|SetIsWieldingWeapon true))))))

(fn ConstructionScript
  (|CallParentFunction)
  (Default|SetEnemyType (Variables|Default|GetBPC_DamageSystem) "NewEnumerator2"))

(fn SetMovementSpeed
  (params (Speed :type E_MovementSpeed%20Enum :default "NewEnumerator0"))
  (Variables|/Script/Engine.CharacterMovementComponent|SetMaxWalkSpeed (Variables|Character|GetCharacterMovement) (Utilities|Select :Index Speed :NewEnumerator0 0.0 :NewEnumerator1 3e+02 :NewEnumerator2 5e+02 :NewEnumerator3 7.5e+02))
  (return 0.0))

(fn GetIdealRange
  (return 6e+02 6e+02))

(fn SelectAnimClassfromType
  (params (EnemyType :type E_EnemyType%20Enum :default "NewEnumerator2"))
  (Components|SkeletalMesh|SetAnimInstanceClass (Variables|Character|GetMesh) (Utilities|Select :Index EnemyType :NewEnumerator2 "/Game/Enemies/02EnemyRanged/Animations/ABP_RRanged.ABP_RRanged_C" :NewEnumerator5 0 :NewEnumerator9 0 :NewEnumerator8 0 :NewEnumerator10 0 :NewEnumerator11 0 :NewEnumerator19 "/Game/Enemies/02EnemyRanged/Animations/ABP_RRanged.ABP_RRanged_C" :NewEnumerator18 "/Game/Enemies/02EnemyRanged/Animations/ABP_RRanged.ABP_RRanged_C" :NewEnumerator20 "/Game/Enemies/02EnemyRanged/Animations/ABP_RRanged.ABP_RRanged_C" :NewEnumerator21 "/Game/Enemies/02EnemyRanged/Animations/ABP_RRanged.ABP_RRanged_C" :NewEnumerator3 0 :NewEnumerator0 0 :NewEnumerator1 0 :NewEnumerator4 0 :NewEnumerator7 0 :NewEnumerator6 "/Game/Enemies/03EnemyMage/Animations/ABP_RMagic.ABP_RMagic_C" :NewEnumerator14 "/Game/Enemies/03EnemyMage/Animations/ABP_RMagic.ABP_RMagic_C" :NewEnumerator13 "/Game/Enemies/03EnemyMage/Animations/ABP_RMagic.ABP_RMagic_C" :NewEnumerator15 "/Game/Enemies/03EnemyMage/Animations/ABP_RMagic.ABP_RMagic_C" :NewEnumerator12 0)))