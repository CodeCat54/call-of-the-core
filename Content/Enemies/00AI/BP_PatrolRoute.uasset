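; BP_PatrolRoute is a spline-based patrol route for enemy AI that tracks a current point along its path.
; IncrementPatrolRoute steps PatrolIndex by Direction and flips Direction at the first and last spline points, so the route runs back and forth rather than looping.
; GetSplinePointAsWorldPosition returns the world location of the current point on the PatrolRoute spline.
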(event Custom|IncrementPatrolRoute
  ;[1 1 1] Increment based on direction 1 or -1
  (bind _output_get (Variables|Default|SetPatrolIndex (+ (Variables|Default|GetPatrolIndex) (Variables|Default|GetDirection))))
  ;[1 1 1] Reverse when end reached
  (if (== _output_get (- (Spline|GetNumberOfSplinePoints (Variables|Default|GetPatrolRoute)) 1))
    (Variables|Default|SetDirection -1)
    (elif (== (Variables|Default|GetPatrolIndex) 0)
      (Variables|Default|SetDirection 1))))

(fn ConstructionScript)

(fn GetSplinePointasWorldPosition
  (return (Spline|GetLocationatSplinePoint (Variables|Default|GetPatrolRoute) (Variables|Default|GetPatrolIndex) "World")))