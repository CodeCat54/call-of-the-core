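; Boss enemy Blueprint that extends a parent enemy class and wields an axe.
; It spawns the axe on BeginPlay and attaches it to a right-hand mesh socket; equip and unequip each wait a tick before signaling completion.
; The construction script seeds the damage system component's max and current health from MaxHealth.
; SetMovementSpeed maps movement states from idle to sprinting onto the character's walk speed.
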(event EventBeginPlay
  (|CallParentFunction)
  (CallFunction|EquipWeapon))

(event EventEquipWeapon
  (bind _returnvalue (Game|SpawnActorfromClass "/Game/Weapons/BP_Weapon_Axe.BP_Weapon_Axe_C" (Math|Transform|MakeTransform "0, 0, 0" "0, 0, 0" "1.000000,1.000000,1.000000") "Undefined" "MultiplyWithRoot" 0 0))
  (bind _output_get (Variables|Default|SetWeaponActor _returnvalue))
  (Transformation|AttachComponentToComponent _output_get (Variables|Character|GetMesh) "Hand_R_Axe_Socket" "KeepRelative" "KeepRelative" "KeepRelative" true)
  (Utilities|FlowControl|DelayUntilNextTick)
  (Default|CallOnWeaponEquipped))

(event EventUnequipWeapon
  (Actor|DestroyActor (Variables|Default|GetWeaponActor))
  (Utilities|FlowControl|DelayUntilNextTick)
  (Default|CallOnWeaponUnequipped))

(fn ConstructionScript
  (bind _bpc_damagesystem (Variables|Default|GetBPC_DamageSystem))
  (|CallParentFunction)
  (bind _output_get (Variables|/Game/DamageSystem/BPC_DamageSystem.BPC_DamageSystem_C|SetMaxHealth _bpc_damagesystem (Variables|Default|GetMaxHealth)))
  (Variables|/Game/DamageSystem/BPC_DamageSystem.BPC_DamageSystem_C|SetCurrentHealth _bpc_damagesystem _output_get))

(fn SetMovementSpeed
  (params (Speed :type E_MovementSpeed%20Enum :default "NewEnumerator0"))
  (bind _output_get (Variables|/Script/Engine.CharacterMovementComponent|SetMaxWalkSpeed (Variables|Character|GetCharacterMovement) (Utilities|Select :Index Speed :NewEnumerator0 0.0 :NewEnumerator1 2.5e+02 :NewEnumerator2 5e+02 :NewEnumerator3 6.5e+02)))
  (return _output_get))