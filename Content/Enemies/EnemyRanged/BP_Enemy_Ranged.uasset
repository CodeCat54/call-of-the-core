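; Ranged enemy child Blueprint that spawns a rifle on BeginPlay, attaches it to its hand socket and fires projectiles at attack targets.
; Attack plays a fire montage whose notify has BPCAttacks launch a randomly typed, random-speed projectile from the weapon, with AttackEnd called on completion or interruption.
; It also sets its damage-system enemy type, maps movement states to walk speeds and reports ideal attack and defend ranges.
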(event EventBeginPlay
  (|CallParentFunction)
  (CallFunction|EquipWeapon))

(event EventAttack
  (params (AttackTarget :type Actor%20Object%20Reference))
  ;[1 1 1] Attack
  (|CallParentFunction AttackTarget)
  (bind _notifyname (Animation|Montage|PlayMontage (Variables|Character|GetMesh) "/Game/Characters/Robot/Animations/RobotRanged/AM_RR_Fire.AM_RR_Fire")
    (:OnCompleted
      (CallFunction|AttackEnd AttackTarget :!label _label))
    (:OnInterrupted
      (goto _label))
    (:OnNotifyBegin
      (switch name _notifyname
        (:Fire
          (Default|ProjectileAttack (Variables|Default|GetBPC_Attacks) (Math|Transform|MakeTransform (Transformation|GetActorLocation (Variables|Default|GetWeaponActor)) "0, 0, 0" "1.000000,1.000000,1.000000") AttackTarget (Utilities|Struct|MakeS_DamageInfo 15.0 "NewEnumerator2" "NewEnumerator0" false false true) (Utilities|Array|Get(acopy) (Variables|Default|GetProjectilesArray) (Math|Random|RandomIntegerinRange 0 3)) (Math|Random|RandomFloatinRange 1e+03 1.5e+03) 0.0 false))))))

(event EventEquipWeapon
  ;[1 1 1] Equip weapon
  (bind _returnvalue (Game|SpawnActorfromClass "/Game/Objects/Weapons/BP_Weapon_Rifle.BP_Weapon_Rifle_C" (Math|Transform|MakeTransform "0, 0, 0") "Undefined" "MultiplyWithRoot" 0 0))
  (bind _output_get (Variables|Default|SetWeaponActor _returnvalue))
  (Transformation|AttachComponentToComponent _output_get (Variables|Character|GetMesh) "Hand_R_Rifle_Socket" "KeepRelative" "KeepRelative" "KeepRelative" true)
  (Variables|Default|SetIsWieldingWeapon true)
  (Default|CallOnWeaponEquipped))

(fn ConstructionScript
  (|CallParentFunction)
  (Default|SetEnemyType (Variables|Default|GetBPC_DamageSystem) "NewEnumerator2"))

(fn SetMovementSpeed
  (params (Speed :type E_MovementSpeed%20Enum :default "NewEnumerator0"))
  (Variables|/Script/Engine.CharacterMovementComponent|SetMaxWalkSpeed (Variables|Character|GetCharacterMovement) (Utilities|Select :Index Speed :NewEnumerator0 0.0 :NewEnumerator1 3e+02 :NewEnumerator2 5e+02 :NewEnumerator3 7.5e+02))
  (return 0.0))

(fn GetIdealRange
  (return 6e+02 6e+02))