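; Sword-wielding robot melee enemy, a child enemy Blueprint with color variants set by EnemyType.
; Construction picks montages per variant and pulls attack stats from DT_EnemyInfoMelee.
; Basic, jump and ground smash attacks delegate to BPCAttacks, while montage notifies drive sword equip and unequip.
; The uninterruptible spin attack uses notifies to spin the mesh by timeline, re-issue AI chase moves and spawn AoE damage limited to the target.
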(event Custom|GroundSmashAttack
  (params (AttackTarget :type Actor%20Object%20Reference))
  ;[1 1 1] Ground smash attack
  (Default|GroundSmash (Variables|Default|GetBPC_Attacks) (Utilities|Struct|MakeS_AttackInfo AttackTarget (Variables|Montages|GetSmashAttackMontage) (Utilities|Struct|MakeS_DamageInfo (Variables|SmashAttack|GetSmashAttackDamage) "NewEnumerator3")) (Variables|SmashAttack|GetSmashAttackRadius) (Variables|SmashAttack|GetSmashAttackOffset) "/Game/Sounds/SFX/SFX_Lightning.SFX_Lightning"))

(event Custom|StopSpinning
  ;[1 1 1] Stop spinning, stop timeline and reset rotation
  (Audio|Components|Audio|Stop (Variables|Default|GetSpinMeshTimeline))
  (Transformation|SetRelativeRotation (Variables|Character|GetMesh) (Variables|SpinAttack|GetMeshRotationBeforeSpin) false false))

(event Custom|AoeSlash
  (params (AttackTarget :type Actor%20Object%20Reference))
  ;[1 1 1] AoE for spin attack
  (bind _returnvalue (Game|SpawnActorfromClass "/Game/Attacks/AoE/BP_Aoe_Base.BP_Aoe_Base_C" (Math|Transform|MakeTransform (Transformation|GetActorLocation) "0, 0, 0" "1.000000,1.000000,1.000000") "Undefined" "MultiplyWithRoot" 0 2e+02 true false false self))
  (Variables|/Game/Attacks/AoE/BP_Aoe_Base.BP_Aoe_Base_C|SetRadius _returnvalue 1.5e+02)
  (EventDispatchers|BindEventtoOnAoeOverlapActor _returnvalue (delegate Custom|AoeDamageActor))
  (Default|Trigger _returnvalue))

(event Custom|AoeDamageActor
  (params (Actor :type Actor%20Object%20Reference))
  ;[1 1 1] AoE for spin attack
  (if (== Actor (stale Custom|AoeSlash AttackTarget))
    (Class|BPIDamageable|TakeDamage(Message) Actor (Utilities|Struct|MakeS_DamageInfo (Variables|SpinAttack|GetSpinAttackDamage) "NewEnumerator1" "NewEnumerator1") self)))

(event Custom|ShortRangeAttack
  (params (AttackTarget :type Actor%20Object%20Reference))
  ;[1 1 1] Short range attack
  (Default|MeleePrimaryAttack (Variables|Default|GetBPC_Attacks) (Utilities|Struct|MakeS_AttackInfo AttackTarget (Variables|Montages|GetBasicAttackMontage) (Utilities|Struct|MakeS_DamageInfo (Variables|BasicAttack|GetBasicAttackDamage) "NewEnumerator1" "NewEnumerator0" false false true true)) 2.0 2e+01 1.0 1.2e+02 "/Game/Sounds/SFX/SFX_SwordSwing.SFX_SwordSwing"))

(event Custom|LongRangeAttack
  (params (AttackTarget :type Actor%20Object%20Reference))
  ;[1 1 1] Long range attack
  (Default|MeleeJumpAttack (Variables|Default|GetBPC_Attacks) (Utilities|Struct|MakeS_AttackInfo AttackTarget (Variables|Montages|GetJumpAttackMontage) (Utilities|Struct|MakeS_DamageInfo (Variables|JumpAttack|GetJumpAttackDamage) "NewEnumerator1" "NewEnumerator0" false false true true)) 1.5 5e+01 1.0 1.2e+02 "/Game/Sounds/SFX/SFX_SwordSwing.SFX_SwordSwing" 2.5e+02 0.85))

(event Custom|SpinAttack
  (params (AttackTarget :type Actor%20Object%20Reference))
  (bind _audio (Variables|Default|GetAudio))
  (bind _bpc_damagesystem (Variables|Default|GetBPC_DamageSystem))
  ;[1 1 1] Spin attack
  (|CallParentFunction AttackTarget)
  (bind _notifyname (Animation|Montage|PlayMontage (Variables|Character|GetMesh) (Variables|Montages|GetSpinAttackMontage))
    (:then
      (Variables|/Game/DamageSystem/BPC_DamageSystem.BPC_DamageSystem_C|SetIsInterruptible _bpc_damagesystem false))
    (:OnCompleted
      (CallFunction|AttackEnd AttackTarget :!label _label)
      (Variables|/Game/DamageSystem/BPC_DamageSystem.BPC_DamageSystem_C|SetIsInterruptible _bpc_damagesystem true)
      (Audio|Components|Audio|FadeOut (Variables|Default|GetAudio) 0.25 0.0 "Linear" :!class /Script/Engine.AudioComponent)
      (CallFunction|StopSpinning))
    (:OnInterrupted
      (goto _label))
    (:OnNotifyBegin
      (switch name _notifyname
        (:Slash
          (Audio|Components|Audio|SetSound _audio "/Game/Sounds/SFX/SFX_SpinAttack.SFX_SpinAttack")
          (Audio|Components|Audio|FadeIn _audio 0.1 1.0 0.0 "Linear" :!class /Script/Engine.AudioComponent))
        (:Spin
          (CallFunction|SpinMesh)
          (CallFunction|ChaseAttackTarget AttackTarget))
        (:AoeSlash
          (CallFunction|AoeSlash AttackTarget))))))

(event Custom|SpinMesh
  ;[1 1 1] Spin mesh
  (Variables|SpinAttack|SetMeshRotationBeforeSpin (Variables|/Script/Engine.SceneComponent|GetRelativeRotation (Variables|Character|GetMesh)))
  (bind _zrotationalpha (Timeline|SpinMeshTimeline PlayFromStart)
    (:Update
      (Transformation|SetRelativeRotation (Variables|Character|GetMesh) (Math|Rotator|MakeRotator (.roll (Variables|SpinAttack|GetMeshRotationBeforeSpin)) (.pitch (Variables|SpinAttack|GetMeshRotationBeforeSpin)) (Math|Float|Lerp (.yaw (Variables|SpinAttack|GetMeshRotationBeforeSpin)) (+ (.yaw (Variables|SpinAttack|GetMeshRotationBeforeSpin)) (|(360*12))) _zrotationalpha)) false false))))

(event Custom|ChaseAttackTarget
  (params (AttackTarget :type Actor%20Object%20Reference))
  ;[1 1 1] Chase attack target for spin attack
  (AI|AIMoveTo self "0, 0, 0" AttackTarget 1.5e+02 false
    (:OnSuccess
      _)
    (:OnFail
      _))
  (Utilities|FlowControl|Delay 0.1)
  (if (Variables|Default|GetAttacking) ; Stop chasing once attack is over
    (CallFunction|ChaseAttackTarget AttackTarget)))

(event EventUnequipWeapon
  ;[1 1 1] Unequip
  (bind _notifyname (Animation|Montage|PlayMontage (Variables|Character|GetMesh) "/Game/Enemies/01EnemyMelee/Animations/AM_RMelee_Sheathe.AM_RMelee_Sheathe")
    (:OnCompleted
      (Default|CallOnWeaponUnequipped))
    (:OnNotifyBegin
      (switch name _notifyname
        (:DropSword
          (Actor|DestroyActor (Variables|Default|GetWeaponActor))
          (Variables|Default|SetIsWieldingWeapon false))
        (:Sheathe
          (CallFunction|PlaySFX "/Game/Sounds/SFX/SFX_SwordSheath.SFX_SwordSheath"))))))

(event EventEquipWeapon
  ;[1 1 1] Equip
  (bind _notifyname (Animation|Montage|PlayMontage (Variables|Character|GetMesh) "/Game/Enemies/01EnemyMelee/Animations/AM_RMelee_Unsheathe.AM_RMelee_Unsheathe")
    (:OnCompleted
      (Default|CallOnWeaponEquipped :!label _label))
    (:OnInterrupted
      (goto _label))
    (:OnNotifyBegin
      (switch name _notifyname
        (:DrawSword
          (bind _returnvalue (Game|SpawnActorfromClass "/Game/Weapons/BP_Weapon_Sword.BP_Weapon_Sword_C" (Transformation|GetActorTransform) "Undefined" "MultiplyWithRoot" 0 (Variables|Default|GetDynamicWeaponMaterial) 0))
          (bind _output_get (Variables|Default|SetWeaponActor _returnvalue))
          (Transformation|AttachComponentToComponent _output_get (Variables|Character|GetMesh) "Hand_R_Sword_Socket" "SnapToTarget" "SnapToTarget" "SnapToTarget" true)
          (Variables|Default|SetIsWieldingWeapon true)
          (CallFunction|PlaySFX "/Game/Sounds/SFX/SFX_SwordDraw.SFX_SwordDraw"))))))

(event EventBeginPlay
  ;[1 1 1] Initialise
  (|CallParentFunction))

(fn ConstructionScript
  (bind _enemytype (Variables|Default|GetEnemyType))
  (|CallParentFunction)
  (Variables|SpinAttack|SetMeshRotationBeforeSpin (Variables|/Script/Engine.SceneComponent|GetRelativeRotation (Variables|Character|GetMesh)))
  (Default|SetEnemyType (Variables|Default|GetBPC_DamageSystem) "NewEnumerator1")
  (CallFunction|SelectVariablesfromType _enemytype)
  (CallFunction|SelectMontagesfromType _enemytype))

(fn GetIdealRange
  (return 1.2e+02 4e+02))

(fn CalculateFutureActorLocation
  (params (Actor :type Actor%20Object%20Reference) (Time :type Float%20%28double-precision%29))
  (bind _returnvalue (Transformation|GetVelocity Actor))
  (bind _returnvalue_2 (* _returnvalue Time))
  (return (+ (Transformation|GetActorLocation Actor) (Math|Vector|MakeVector (.x _returnvalue_2) (.y _returnvalue_2) 0.0))))

(fn SelectVariablesfromType
  (params (EnemyType :type E_EnemyType%20Enum :default "NewEnumerator2"))
  (bind _returnvalue (Utilities|GetDataTableRow "/Game/DataTables/DT_EnemyInfoMelee.DT_EnemyInfoMelee" (Utilities|String|StringToName (Utilities|String|EnumtoString EnemyType)))
    (:then
      (Utilities|FlowControl|Sequence
        (:then_0
          (Variables|BasicAttack|SetBasicAttackDamage (.basicattackdamage _returnvalue)))
        (:then_1
          (Variables|JumpAttack|SetJumpAttackDamage (.jumpattackdamage _returnvalue)))
        (:then_2
          (Variables|SpinAttack|SetSpinAttackDamage (.spinattackdamage _returnvalue)))
        (:then_3
          (Variables|SmashAttack|SetSmashAttackDamage (.smashattackdamage _returnvalue)))
        (:then_4
          (Variables|SmashAttack|SetSmashAttackRadius (.smashattackradius _returnvalue)))
        (:then_5
          (Variables|SmashAttack|SetSmashAttackOffset (.smashattackoffset _returnvalue)))))))

(fn SelectMaterialfromType0
  (params (EnemyType :type E_EnemyType%20Enum :default "NewEnumerator2"))
  (Rendering|Material|SetMaterial (Variables|Character|GetMesh) 0 (Utilities|Select :Index EnemyType :NewEnumerator2 "/Game/Materials/Enemies/MI_RobotMeleeRed.MI_RobotMeleeRed" :NewEnumerator5 "/Game/Materials/Enemies/MI_RobotMeleeYellow.MI_RobotMeleeYellow" :NewEnumerator9 "/Game/Materials/Enemies/MI_RobotMeleeBlue.MI_RobotMeleeBlue" :NewEnumerator8 "/Game/Materials/Enemies/MI_RobotMeleeWhite.MI_RobotMeleeWhite" :NewEnumerator10 "/Game/Materials/Enemies/MI_RobotMeleePurple.MI_RobotMeleePurple" :NewEnumerator11 "/Game/Materials/Enemies/MI_RobotMeleeRed.MI_RobotMeleeRed" :NewEnumerator19 0 :NewEnumerator18 0 :NewEnumerator20 0 :NewEnumerator21 0 :NewEnumerator3 0 :NewEnumerator0 0 :NewEnumerator1 0 :NewEnumerator4 0 :NewEnumerator7 0 :NewEnumerator6 0 :NewEnumerator14 0 :NewEnumerator13 0 :NewEnumerator15 0 :NewEnumerator12 0)))

(fn SelectMontagesfromType
  (params (EnemyType :type E_EnemyType%20Enum :default "NewEnumerator2"))
  (Variables|Montages|SetBasicAttackMontage (Utilities|Select :Index EnemyType :NewEnumerator2 "/Game/Enemies/01EnemyMelee/Animations/BasicAttack/AM_RMelee_AttackRed.AM_RMelee_AttackRed" :NewEnumerator5 "/Game/Enemies/01EnemyMelee/Animations/BasicAttack/AM_RMelee_AttackYellow.AM_RMelee_AttackYellow" :NewEnumerator9 "/Game/Enemies/01EnemyMelee/Animations/BasicAttack/AM_RMelee_AttackBlue.AM_RMelee_AttackBlue" :NewEnumerator8 "/Game/Enemies/01EnemyMelee/Animations/BasicAttack/AM_RMelee_AttackWhite.AM_RMelee_AttackWhite" :NewEnumerator10 "/Game/Enemies/01EnemyMelee/Animations/BasicAttack/AM_RMelee_AttackPurple.AM_RMelee_AttackPurple" :NewEnumerator11 "/Game/Enemies/01EnemyMelee/Animations/BasicAttack/AM_RMelee_AttackRed.AM_RMelee_AttackRed" :NewEnumerator19 0 :NewEnumerator18 0 :NewEnumerator20 0 :NewEnumerator21 0 :NewEnumerator3 0 :NewEnumerator0 0 :NewEnumerator1 0 :NewEnumerator4 0 :NewEnumerator7 0 :NewEnumerator6 0 :NewEnumerator14 0 :NewEnumerator13 0 :NewEnumerator15 0 :NewEnumerator12 0))
  (Variables|Montages|SetJumpAttackMontage (Utilities|Select :Index EnemyType :NewEnumerator2 "/Game/Enemies/01EnemyMelee/Animations/JumpAttack/AM_RMelee_JumpAttackRed.AM_RMelee_JumpAttackRed" :NewEnumerator5 "/Game/Enemies/01EnemyMelee/Animations/JumpAttack/AM_RMelee_JumpAttackYellow.AM_RMelee_JumpAttackYellow" :NewEnumerator9 "/Game/Enemies/01EnemyMelee/Animations/JumpAttack/AM_RMelee_JumpAttackBlue.AM_RMelee_JumpAttackBlue" :NewEnumerator8 "/Game/Enemies/01EnemyMelee/Animations/JumpAttack/AM_RMelee_JumpAttackWhite.AM_RMelee_JumpAttackWhite" :NewEnumerator10 "/Game/Enemies/01EnemyMelee/Animations/JumpAttack/AM_RMelee_JumpAttackPurple.AM_RMelee_JumpAttackPurple" :NewEnumerator11 "/Game/Enemies/01EnemyMelee/Animations/JumpAttack/AM_RMelee_JumpAttackRed.AM_RMelee_JumpAttackRed" :NewEnumerator19 0 :NewEnumerator18 0 :NewEnumerator20 0 :NewEnumerator21 0 :NewEnumerator3 0 :NewEnumerator0 0 :NewEnumerator1 0 :NewEnumerator4 0 :NewEnumerator7 0 :NewEnumerator6 0 :NewEnumerator14 0 :NewEnumerator13 0 :NewEnumerator15 0 :NewEnumerator12 0))
  (Variables|Montages|SetSpinAttackMontage (Utilities|Select :Index EnemyType :NewEnumerator2 "/Game/Enemies/01EnemyMelee/Animations/SpinAttack/AM_RMelee_SpinAttackRed.AM_RMelee_SpinAttackRed" :NewEnumerator5 "/Game/Enemies/01EnemyMelee/Animations/SpinAttack/AM_RMelee_SpinAttackYellow.AM_RMelee_SpinAttackYellow" :NewEnumerator9 "/Game/Enemies/01EnemyMelee/Animations/SpinAttack/AM_RMelee_SpinAttackBlue.AM_RMelee_SpinAttackBlue" :NewEnumerator8 "/Game/Enemies/01EnemyMelee/Animations/SpinAttack/AM_RMelee_SpinAttackWhite.AM_RMelee_SpinAttackWhite" :NewEnumerator10 "/Game/Enemies/01EnemyMelee/Animations/SpinAttack/AM_RMelee_SpinAttackPurple.AM_RMelee_SpinAttackPurple" :NewEnumerator11 "/Game/Enemies/01EnemyMelee/Animations/SpinAttack/AM_RMelee_SpinAttackRed.AM_RMelee_SpinAttackRed" :NewEnumerator19 0 :NewEnumerator18 0 :NewEnumerator20 0 :NewEnumerator21 0 :NewEnumerator3 0 :NewEnumerator0 0 :NewEnumerator1 0 :NewEnumerator4 0 :NewEnumerator7 0 :NewEnumerator6 0 :NewEnumerator14 0 :NewEnumerator13 0 :NewEnumerator15 0 :NewEnumerator12 0))
  (Variables|Montages|SetSmashAttackMontage (Utilities|Select :Index EnemyType :NewEnumerator2 "/Game/Enemies/01EnemyMelee/Animations/SmashAttack/AM_RMelee_GroundSmashRed.AM_RMelee_GroundSmashRed" :NewEnumerator5 "/Game/Enemies/01EnemyMelee/Animations/SmashAttack/AM_RMelee_GroundSmashYellow.AM_RMelee_GroundSmashYellow" :NewEnumerator9 "/Game/Enemies/01EnemyMelee/Animations/SmashAttack/AM_RMelee_GroundSmashBlue.AM_RMelee_GroundSmashBlue" :NewEnumerator8 "/Game/Enemies/01EnemyMelee/Animations/SmashAttack/AM_RMelee_GroundSmashWhite.AM_RMelee_GroundSmashWhite" :NewEnumerator10 "/Game/Enemies/01EnemyMelee/Animations/SmashAttack/AM_RMelee_GroundSmashPurple.AM_RMelee_GroundSmashPurple" :NewEnumerator11 "/Game/Enemies/01EnemyMelee/Animations/SmashAttack/AM_RMelee_GroundSmashRed.AM_RMelee_GroundSmashRed" :NewEnumerator19 0 :NewEnumerator18 0 :NewEnumerator20 0 :NewEnumerator21 0 :NewEnumerator3 0 :NewEnumerator0 0 :NewEnumerator1 0 :NewEnumerator4 0 :NewEnumerator7 0 :NewEnumerator6 0 :NewEnumerator14 0 :NewEnumerator13 0 :NewEnumerator15 0 :NewEnumerator12 0)))