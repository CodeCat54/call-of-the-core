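; BP_Aoe_Blast_Base is a base AoE blast actor that adds visual and audio feedback when triggered.
; Its Trigger override runs the parent logic, then spawns the blast particle effect attached to the root and plays the blast sound at the actor's location.
; The actor destroys itself when the particle system finishes, or after a short delay if no effect is set.
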(event Custom|SystemFinished
  (params (PSystem :type Particle%20System%20Component%20Object%20Reference))
  ;[1 1 1] FX
  (Actor|DestroyActor))

(event Custom|SpawnBlastEffect
  ;[1 1 1] FX
  (bind _blasteffect (Variables|Default|GetBlastEffect)
    (:then
      (bind _returnvalue (Effects|SpawnEmitterAttached _blasteffect (Variables|Transformation|GetRootComponent) "None"))
      (EventDispatchers|BindEventtoOnSystemFinished _returnvalue (delegate Custom|SystemFinished)))
    (:else
      (Utilities|FlowControl|Delay 1.0)
      (Actor|DestroyActor))))

(event Custom|PlayBlastSound
  ;[1 1 1] Sound
  (bind _blastsound (Variables|Default|GetBlastSound)
    (:then
      (Audio|PlaySoundatLocation _blastsound (Transformation|GetActorLocation) "0, 0, 0" 1.0 1.0 0.0 0 0 0 0))
    (:else)))

(event EventTrigger
  ;[1 1 1] Trigger override
  (|CallParentFunction)
  (CallFunction|SpawnBlastEffect)
  (CallFunction|PlayBlastSound))

(fn ConstructionScript
  (|CallParentFunction))