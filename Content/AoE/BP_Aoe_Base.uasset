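; Base area-of-effect actor that finds pawns within a radius and reports each through the OnAoeOverlapActor dispatcher.
; Trigger runs the sphere overlap at the actor's location, optionally ignoring the instigator and drawing a debug sphere, and prints each hit actor's name.
; It fires manually or on BeginPlay, where a short delay lets listeners bind first.
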(event Custom|SpawnAoeSphere
  ;[1 1 1] Spawn sphere
  (if (Variables|Default|GetDrawDebugSphere)
    (Rendering|Debug|DrawDebugSphere (Transformation|GetActorLocation) (Variables|Default|GetRadius) 12 "(R=0.922740,G=0.000000,B=1.000000,A=1.000000)" 2.0 1.0))
  (bind _outactors (Collision|SphereOverlapActors (Transformation|GetActorLocation) (Variables|Default|GetRadius) (Utilities|Array|MakeArray "ObjectTypeQuery3") 0 (select (Variables|Default|GetIgnoreInstigator) (Utilities|Array|MakeArray (Game|GetInstigator)) 0)))
  (for _array_element _outactors
    (Default|CallOnAoeOverlapActor _array_element)
    (Development|PrintString (Utilities|GetDisplayName _array_element))))

(event Custom|Trigger
  ;[1 1 1] Manual trigger
  (CallFunction|SpawnAoeSphere))

(event EventBeginPlay
  ;[1 1 1] Trigger on begin play, delay to allow binding
  (if (Variables|Default|GetTriggerOnBeginPlay)
    (Utilities|FlowControl|Delay 0.2)
    (CallFunction|Trigger)))

(fn ConstructionScript)