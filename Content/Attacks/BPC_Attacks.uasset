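; Attack component that gives its owning character melee, long-range leap, ground smash and mage projectile attacks.
; Each attack plays a montage whose notifies trigger sphere traces, AoE actors, projectiles or an arced launch, messaging the owner on interruptibility and attack end.
; A separate bullet event uses line traces.
; Damage goes through interface messages filtered by team number, with bullet and projectile hits also reported as damage events.
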(event Custom|ProjectileAttack
  (params (SpawnTransform :type Transform) (Target :type Actor%20Object%20Reference) (DamageInfo :type S%20Damage%20Info%20Structure) (ProjectileType :type BP%20Projectile%20Base%20Class%20Reference) (Speed :type Float%20%28double-precision%29) (Gravity :type Float%20%28double-precision%29) (IsHoming :type Boolean))
  ;[1 1 1] Variable projectile attack notify
  (bind _returnvalue (Game|SpawnActorfromClass ProjectileType SpawnTransform "Undefined" "MultiplyWithRoot" (Components|GetOwner) Speed Gravity Target IsHoming 0))
  (EventDispatchers|BindEventtoOnProjectileImpact _returnvalue (delegate Custom|OnProjectileHit))
  (Collision|IgnoreActorwhenMoving (Actor|GetComponentbyClass (Components|GetOwner) "/Script/Engine.CapsuleComponent") _returnvalue true))

(event Custom|OnProjectileHit
  (params (OtherActor :type Actor%20Object%20Reference) (Hit :type Hit%20Result%20Structure))
  (bind _returnvalue (Components|GetOwner))
  ;[1 1 1] Variable projectile attack notify
  (bind _damagedealt (CallFunction|DamageSingleNonTeamMember Hit (stale Custom|ProjectileAttack DamageInfo)))
  (if _damagedealt
    (Class|AISenseDamage|ReportDamageEvent OtherActor _returnvalue (.DamageAmount (Utilities|Struct|BreakS_DamageInfo (stale Custom|ProjectileAttack DamageInfo))) (Transformation|GetActorLocation _returnvalue) "0, 0, 0" "None")))

(event Custom|AoeDamage
  (params (Radius :type Float%20%28single-precision%29) (DamageInfo :type S%20Damage%20Info%20Structure) (Offset :type Float%20%28double-precision%29))
  (bind _returnvalue (Components|GetOwner))
  ;[1 1 1] AoE damage notify
  (bind _returnvalue_2 (Game|SpawnActorfromClass "/Game/Attacks/AoE/BP_Aoe_Base.BP_Aoe_Base_C" (Math|Transform|MakeTransform (+ (Transformation|GetActorLocation _returnvalue) (* (Transformation|GetActorForwardVector _returnvalue) Offset)) "0, 0, 0" "1.000000,1.000000,1.000000") "Undefined" "MultiplyWithRoot" 0 true false false (.AsPawn (Utilities|Casting|CastToPawn _returnvalue))))
  (Variables|/Game/Attacks/AoE/BP_Aoe_Base.BP_Aoe_Base_C|SetRadius _returnvalue_2 Radius)
  (EventDispatchers|BindEventtoOnAoeOverlapActor _returnvalue_2 (delegate Custom|AoeDamageActor))
  (Default|Trigger _returnvalue_2))

(event Custom|AoeDamageActor
  (params (Actor :type Actor%20Object%20Reference))
  (bind _returnvalue (Components|GetOwner))
  ;[1 1 1] AoE damage notify
  (bind _teamnumber (Class|BPIDamageable|GetTeamNumber(Message) Actor))
  (bind _teamnumber_2 (Class|BPIDamageable|GetTeamNumber(Message) _returnvalue))
  (if (!= _teamnumber_2 _teamnumber) ; Only damage actors on\nother team
    (Class|BPIDamageable|TakeDamage(Message) Actor (stale Custom|AoeDamage DamageInfo) _returnvalue)))

(event Custom|FireBullet
  (params (TraceStart :type Vector) (TraceEnd :type Vector) (DamageInfo :type S%20Damage%20Info%20Structure))
  (bind _returnvalue (Components|GetOwner))
  ;[1 1 1] Bullet line trace notify
  (bind (_outhits _returnvalue_2) (Class|KismetSystemLibrary|LineTraceMultiforObjects TraceStart TraceEnd (Utilities|Array|MakeArray "ObjectTypeQuery3") false (Utilities|Array|MakeArray (Components|GetOwner)) "ForDuration" true))
  (if _returnvalue_2
    (bind _damagedactor (CallFunction|DamageFirstNonTeamMember _outhits DamageInfo))
    (Class|AISenseDamage|ReportDamageEvent _damagedactor _returnvalue (.DamageAmount (Utilities|Struct|BreakS_DamageInfo DamageInfo)) (Transformation|GetActorLocation _returnvalue) "0, 0, 0" "None")))

(event Custom|GroundSmash
  (params (AttackInfo :type S%20Attack%20Info%20Structure) (Radius :type Float%20%28single-precision%29) (Offset :type Float%20%28double-precision%29))
  (bind _returnvalue (Components|GetOwner))
  ;[1 1 1] Ground smash
  (bind _mesh (CallFunction|AttackBase))
  (bind _notifyname (Animation|Montage|PlayMontage _mesh (.montage AttackInfo))
    (:then
      (Class|BPIDamageable|SetIsInterruptible(Message) _returnvalue false))
    (:OnCompleted
      (Class|BPIEnemyAI|AttackEnd(Message) _returnvalue (.attacktarget AttackInfo) :!label _label)
      (Class|BPIDamageable|SetIsInterruptible(Message) _returnvalue true))
    (:OnInterrupted
      (goto _label))
    (:OnNotifyBegin
      (switch name _notifyname
        (:Smash
          (CallFunction|AoeDamage Radius (.damageinfo AttackInfo) Offset))))))

(event Custom|LongRangeMeleeAttack
  (params (AttackInfo :type S%20Attack%20Info%20Structure) (Radius :type Float%20%28single-precision%29) (Length :type Float%20%28single-precision%29))
  (bind _returnvalue (Components|GetOwner))
  ;[1 1 1] Long range melee attack
  (bind _mesh (CallFunction|AttackBase))
  (bind _notifyname (Animation|Montage|PlayMontage _mesh (.montage AttackInfo) 1.5)
    (:then
      (Class|BPIDamageable|SetIsInterruptible(Message) _returnvalue false))
    (:OnCompleted
      (Class|BPIEnemyAI|AttackEnd(Message) _returnvalue (.attacktarget AttackInfo) :!label _label)
      (Class|BPIDamageable|SetIsInterruptible(Message) _returnvalue true))
    (:OnInterrupted
      (goto _label))
    (:OnNotifyBegin
      (switch name _notifyname
        (:Slash
          (CallFunction|SphereTraceDamage (.damageinfo AttackInfo) Radius Length))
        (:Jump
          (CallFunction|JumptoAttackTarget (.attacktarget AttackInfo)))))))

(event Custom|OnLand
  (params (Hit :type Hit%20Result%20Structure%20%28by%20ref%29))
  (bind _returnvalue (Components|GetOwner))
  (bind _ascharacter (Utilities|Casting|CastToCharacter _returnvalue))
  ;[1 1 1] Jump to attack target
  (EventDispatchers|UnbindEventfromLandedDelegate _ascharacter (delegate Custom|OnLand))
  (Components|Movement|StopMovementImmediately (Variables|/Script/Engine.Character|GetCharacterMovement _ascharacter)))

(event Custom|PrimaryMeleeAttack
  (params (AttackInfo :type S%20Attack%20Info%20Structure) (Radius :type Float%20%28double-precision%29) (Length :type Float%20%28double-precision%29))
  (bind _returnvalue (Components|GetOwner))
  ;[1 1 1] Primary melee attack
  (bind _mesh (CallFunction|AttackBase))
  (bind _notifyname (Animation|Montage|PlayMontage _mesh (.montage AttackInfo) 2.0)
    (:then
      (Class|BPIDamageable|SetIsInterruptible(Message) _returnvalue false))
    (:OnCompleted
      (Class|BPIEnemyAI|AttackEnd(Message) _returnvalue (.attacktarget AttackInfo) :!label _label)
      (Class|BPIDamageable|SetIsInterruptible(Message) _returnvalue true))
    (:OnInterrupted
      (goto _label))
    (:OnNotifyBegin
      (switch name _notifyname
        (:Slash
          (CallFunction|SphereTraceDamage (.damageinfo AttackInfo) Radius Length))))))

(event Custom|SphereTraceDamage
  (params (DamageInfo :type S%20Damage%20Info%20Structure) (Radius :type Float%20%28single-precision%29) (Length :type Float%20%28single-precision%29))
  (bind _returnvalue (Components|GetOwner))
  (bind _returnvalue_2 (Transformation|GetActorLocation _returnvalue))
  ;[1 1 1] Sphere trace notify
  (bind (_outhits _returnvalue_3) (Collision|MultiSphereTraceForObjects _returnvalue_2 (+ _returnvalue_2 (* (Transformation|GetActorForwardVector _returnvalue) Length)) Radius (Utilities|Array|MakeArray "ObjectTypeQuery3") false 0 "None"))
  (if _returnvalue_3
    (CallFunction|DamageAllNonTeamMembers self _outhits DamageInfo)))

(event Custom|JumpToAttackTarget
  (params (AttackTarget :type Actor%20Object%20Reference))
  (bind _returnvalue (Components|GetOwner))
  (bind _returnvalue_2 (Transformation|GetActorLocation AttackTarget))
  (bind _ascharacter (Utilities|Casting|CastToCharacter _returnvalue))
  ;[1 1 1] Jump to attack target
  (bind _outlaunchvelocity (Game|SuggestProjectileVelocityCustomArc (Transformation|GetActorLocation (Components|GetOwner)) (Math|Vector|MakeVector (.x _returnvalue_2) (.y _returnvalue_2) (+ (.z _returnvalue_2) 2.5e+02)) 0.0 0.85))
  (Character|LaunchCharacter _ascharacter _outlaunchvelocity false true)
  (EventDispatchers|AssignLandedDelegate _ascharacter (delegate Custom|OnLand)))

(event Custom|BasicMageAttack
  (params (AttackInfo :type S%20Attack%20Info%20Structure) (ProjectileType :type BP%20Projectile%20Base%20Class%20Reference) (Speed :type Float%20%28double-precision%29) (Gravity :type Float%20%28double-precision%29) (IsHoming :type Boolean))
  (bind _returnvalue (Components|GetOwner))
  ;[1 1 1] Basic mage attack
  (bind _mesh (CallFunction|AttackBase))
  (bind _notifyname (Animation|Montage|PlayMontage _mesh (.montage AttackInfo) 1.5)
    (:then
      (Class|BPIDamageable|SetIsInterruptible(Message) _returnvalue false))
    (:OnCompleted
      (Class|BPIEnemyAI|AttackEnd(Message) _returnvalue (.attacktarget AttackInfo) :!label _label)
      (Class|BPIDamageable|SetIsInterruptible(Message) _returnvalue true))
    (:OnInterrupted
      (goto _label))
    (:OnNotifyBegin
      (switch name _notifyname
        (:Fire
          (CallFunction|ProjectileAttack (Math|Transform|MakeTransform (Transformation|GetSocketLocation _mesh "RightHand") "0, 0, 0" "1.000000,1.000000,1.000000") (.attacktarget AttackInfo) (.damageinfo AttackInfo) ProjectileType Speed Gravity IsHoming))))))

(event Custom|MageBarrageAttack
  (params (AttackInfo :type S%20Attack%20Info%20Structure) (ProjectileType :type BP%20Projectile%20Base%20Class%20Reference) (Speed :type Float%20%28double-precision%29) (Gravity :type Float%20%28double-precision%29) (IsHoming :type Boolean))
  (bind _returnvalue (Components|GetOwner))
  ;[1 1 1] Mage barrage attack
  (bind _mesh (CallFunction|AttackBase))
  (bind _notifyname (Animation|Montage|PlayMontage _mesh (.montage AttackInfo))
    (:OnCompleted
      (Class|BPIEnemyAI|AttackEnd(Message) _returnvalue (.attacktarget AttackInfo) :!label _label)
      (Class|BPIDamageable|SetIsInterruptible(Message) _returnvalue true))
    (:OnInterrupted
      (goto _label))
    (:OnNotifyBegin
      (switch name _notifyname
        (:Fire
          (CallFunction|ProjectileAttack (Math|Transform|MakeTransform (Transformation|GetSocketLocation _mesh "RightHand") (Math|Rotator|FindLookatRotation (Transformation|GetActorLocation (Components|GetOwner)) (+ (Transformation|GetActorLocation (.attacktarget AttackInfo)) (Math|Vector|MakeVector 0.0 (Math|Random|RandomFloatinRange -3e+02 3e+02) 0.0))) "1.000000,1.000000,1.000000") 0 (.damageinfo AttackInfo) ProjectileType Speed Gravity IsHoming)
          (Class|BPIDamageable|SetIsInterruptible(Message) _returnvalue false))))))

(fn DamageAllNonTeamMembers
  (params (Hits :type Array%20of%20Hit%20Result%20Structures) (DamageInfo :type S%20Damage%20Info%20Structure))
  (bind _returnvalue (Components|GetOwner))
  (for _array_element Hits
    (bind _teamnumber (Class|BPIDamageable|GetTeamNumber(Message) (.HitActor (Collision|BreakHitResult _array_element))))
    (bind _teamnumber_2 (Class|BPIDamageable|GetTeamNumber(Message) _returnvalue))
    (if (and (!= _teamnumber_2 _teamnumber) (not (Utilities|Array|ContainsItem (LocalVariables|GetActorsDamagedSoFar) (.HitActor (Collision|BreakHitResult _array_element)))))
      (Class|BPIDamageable|TakeDamage(Message) (.HitActor (Collision|BreakHitResult _array_element)) DamageInfo _returnvalue)
      (Utilities|Array|AddUnique (LocalVariables|GetActorsDamagedSoFar) (.HitActor (Collision|BreakHitResult _array_element)))))
  (return (LocalVariables|GetActorsDamagedSoFar)))

(fn DamageFirstNonTeamMember
  (params (Hits :type Array%20of%20Hit%20Result%20Structures) (DamageInfo :type S%20Damage%20Info%20Structure))
  (bind _array_element (Utilities|Array|ForEachLoopwithBreak Hits :!label _label)
    (:LoopBody
      (bind _teamnumber (Class|BPIDamageable|GetTeamNumber(Message) (Components|GetOwner)))
      (bind _teamnumber_2 (Class|BPIDamageable|GetTeamNumber(Message) (.HitActor (Collision|BreakHitResult _array_element))))
      (if (!= _teamnumber_2 _teamnumber)
        (Class|BPIDamageable|TakeDamage(Message) (.HitActor (Collision|BreakHitResult _array_element)) DamageInfo)
        (Utilities|FlowControl|Sequence
          (:then_0
            (goto _label Break))
          (:then_1
            (return (.HitActor (Collision|BreakHitResult _array_element)))))))))

(fn DamageSingleNonTeamMember
  (params (Hit :type Hit%20Result%20Structure) (DamageInfo :type S%20Damage%20Info%20Structure))
  (bind _hitactor (Collision|BreakHitResult Hit))
  (bind _returnvalue (Components|GetOwner))
  (bind _teamnumber (Class|BPIDamageable|GetTeamNumber(Message) _hitactor))
  (bind _teamnumber_2 (Class|BPIDamageable|GetTeamNumber(Message) _returnvalue))
  (if (!= _teamnumber_2 _teamnumber)
    (Class|BPIDamageable|TakeDamage(Message) _hitactor DamageInfo _returnvalue)
    (return true)
    (else
      (return false))))

(fn AttackBase
  (bind _returnvalue (Components|GetOwner))
  ;[1 1 1] Run parent attack function, return mesh
  (Class|BPIEnemyAI|Attack(Message) _returnvalue) ; Set attacking to true
  (bind _ascharacter (Utilities|Casting|CastToCharacter _returnvalue))
  (return (Variables|/Script/Engine.Character|GetMesh _ascharacter)))

(fn CalculateFutureActorLocation
  (params (Actor :type Actor%20Object%20Reference) (Time :type Float%20%28double-precision%29))
  (bind _returnvalue (Transformation|GetVelocity Actor))
  (bind _returnvalue_2 (* _returnvalue Time))
  (return (+ (Transformation|GetActorLocation Actor) (Math|Vector|MakeVector (.x _returnvalue_2) (.y _returnvalue_2) 0.0))))